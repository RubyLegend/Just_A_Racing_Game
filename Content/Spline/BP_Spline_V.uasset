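; BP_Spline_V is an actor that builds a spline, apparently a road path, from the Road_tr_csv data table.
; On construction, CreatePoints clears the spline and adds one point per row, scaled and offset by the actor's location without applying its rotation.
; Each row's left and right handle positions become arrive and leave tangents, using the factor-of-three Bezier-to-Hermite conversion to reproduce the imported curve.
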(event EventBeginPlay)

(event Collision|EventActorBeginOverlap
  (params (OtherActor :type Actor%20Object%20Reference)))

(event EventTick
  (params (DeltaSeconds :type Float%20%28single-precision%29)))

(fn ConstructionScript
  (CallFunction|CreatePoints))

(fn CreatePoints
  (bind _newlocalvar_1 (LocalVariables|GetNewLocalVar_1))
  (Spline|ClearSplinePoints (Variables|Default|GetSpline) true)
  (bind _outrownames (DataTable|GetDataTableRowNames "/Game/Spline/road_tr_csv.road_tr_csv"))
  (for (_array_element _array_index) _outrownames
    (bind _returnvalue (Utilities|GetDataTableRow "/Game/Spline/road_tr_csv.road_tr_csv" _array_element)
      (:then
        (Spline|AddSplinePoint (Variables|Default|GetSpline) (+ (Transformation|GetActorLocation) (* (Math|Vector|MakeVector (.px (Utilities|Struct|BreakSplineStruct _returnvalue)) (.py (Utilities|Struct|BreakSplineStruct _returnvalue)) (.pz (Utilities|Struct|BreakSplineStruct _returnvalue))) _newlocalvar_1)) "World" true)
        (Spline|SetTangentsatSplinePoint (Variables|Default|GetSpline) _array_index (* (- (+ (Transformation|GetActorLocation) (* (Math|Vector|MakeVector (.px (Utilities|Struct|BreakSplineStruct _returnvalue)) (.py (Utilities|Struct|BreakSplineStruct _returnvalue)) (.pz (Utilities|Struct|BreakSplineStruct _returnvalue))) _newlocalvar_1)) (+ (Transformation|GetActorLocation) (* (Math|Vector|MakeVector (.hlx (Utilities|Struct|BreakSplineStruct _returnvalue)) (.hly (Utilities|Struct|BreakSplineStruct _returnvalue)) (.hlz (Utilities|Struct|BreakSplineStruct _returnvalue))) _newlocalvar_1))) 3.0) (* (- (+ (Transformation|GetActorLocation) (* (Math|Vector|MakeVector (.hrx (Utilities|Struct|BreakSplineStruct _returnvalue)) (.hry (Utilities|Struct|BreakSplineStruct _returnvalue)) (.hrz (Utilities|Struct|BreakSplineStruct _returnvalue))) _newlocalvar_1)) (+ (Transformation|GetActorLocation) (* (Math|Vector|MakeVector (.px (Utilities|Struct|BreakSplineStruct _returnvalue)) (.py (Utilities|Struct|BreakSplineStruct _returnvalue)) (.pz (Utilities|Struct|BreakSplineStruct _returnvalue))) _newlocalvar_1))) 3.0) "World" true)))))