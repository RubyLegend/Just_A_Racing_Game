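; Player-driven car Blueprint that routes throttle, brake, steering and handbrake input to its vehicle movement component, with handbrake toggling rear lights.
; Tick ramps a smoothed value from forward speed and last gas input into the Engine's RPM parameter.
; Nitro activates a physics thruster while held.
; MouseX and MouseY share spring-arm rotation logic, which resets the camera from actor rotation with downward pitch after an idle delay.
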(event EventTick
  (params (DeltaSeconds :type Float%20%28single-precision%29))
  (bind _spad (Variables|Default|Getspad))
  (bind _rost (Variables|Default|Getrost))
  (bind _vehiclemovementcomponent (Variables|Default|GetVehicleMovementComponent))
  (bind _engine (Variables|Default|GetEngine))
  (bind _returnvalue (Vehicle|GetForwardSpeed _vehiclemovementcomponent))
  (bind _returnvalue_2 (Math|Float|Absolute(Float) _returnvalue))
  (bind _returnvalue_3 (> _returnvalue_2 1e+02))
  (bind _returnvalue_4 (select _returnvalue_3 1e+02 _returnvalue_2))
  (bind _output_get (Variables|Default|SetCamera%20Movement%20Delta (+ DeltaSeconds (stale _output_get))))
  (Class|AudioParameterControllerInterface|ResetParameters _engine)
  (bind _output_get_2 (Variables|Default|Setsp (select (> (Variables|Default|Getlast_gas) 0.0) (select (> (- _returnvalue_2 (Variables|Default|Getsp)) _rost) (+ (Variables|Default|Getsp) _rost) _returnvalue_2) (select (> (Variables|Default|Getsp) (+ _spad _returnvalue_4)) (- (Variables|Default|Getsp) _spad) _returnvalue_4))))
  (Audio|Parameter|SetFloatParameter _engine "RPM" _output_get_2 :!class /Script/Engine.AudioComponent))

(event Input|ActionEvents|InputActionHandBrake
  (params (Key :type Key%20Structure :default "None"))
  (bind _vehiclemovementcomponent (Variables|Default|GetVehicleMovementComponent))
  (bind _mesh (Variables|Character|GetMesh))
  (bind _rl_light (Variables|Default|GetRL%20Light))
  ;[1 1 1] HandBrake
  (:Pressed
    (Class|ChaosVehicleMovementComponent|SetHandbrakeInput _vehiclemovementcomponent true)
    (Rendering|Material|SetMaterial _mesh 1 "/Game/ARCADE_FREE_Racing_Car/TestImport/BackLights_on.BackLights_on")
    (Rendering|SetVisibility _rl_light true false))
  (:Released
    (Class|ChaosVehicleMovementComponent|SetHandbrakeInput _vehiclemovementcomponent false)
    (Rendering|Material|SetMaterial _mesh 1 "/Game/ARCADE_FREE_Racing_Car/TestImport/BackLights_off.BackLights_off")
    (Rendering|SetVisibility _rl_light false false)))

(event Input|ActionEvents|InputActionNitroBoost
  (params (Key :type Key%20Structure :default "None"))
  (bind _physicsthruster (Variables|Default|GetPhysicsThruster))
  (bind _vehiclemovementcomponent (Variables|Default|GetVehicleMovementComponent))
  (bind _returnvalue (Vehicle|GetForwardSpeed _vehiclemovementcomponent))
  (bind _returnvalue_2 (Class|MovementComponent|GetMaxSpeed _vehiclemovementcomponent))
  (bind _returnvalue_3 (+ _returnvalue_2 2e+06))
  (bind _returnvalue_4 (+ _returnvalue 2e+06))
  (:Pressed
    (Development|PrintText "Thrust enabled")
    (Variables|/Script/Engine.PhysicsThrusterComponent|SetThrustStrength _physicsthruster (Math|Float|SelectFloat _returnvalue_3 _returnvalue_4 (> _returnvalue_4 _returnvalue_3)))
    (Components|Activation|Activate _physicsthruster false))
  (:Released
    (Development|PrintText "Thrust disabled")
    (Variables|/Script/Engine.PhysicsThrusterComponent|SetThrustStrength _physicsthruster 0.0)
    (Components|Activation|Deactivate _physicsthruster)))

(event Input|AxisEvents|InputAxisGas
  (params (AxisValue :type Float%20%28single-precision%29))
  ;[1 1 1] Gas
  (Class|ChaosVehicleMovementComponent|SetThrottleInput (Variables|Default|GetVehicleMovementComponent) AxisValue)
  (Variables|Default|SetLast_Gas (Math|Float|Absolute(Float) AxisValue)))

(event Input|AxisEvents|InputAxisReverseGas
  (params (AxisValue :type Float%20%28single-precision%29))
  ;[1 1 1] Gas
  (Class|ChaosVehicleMovementComponent|SetBrakeInput (Variables|Default|GetVehicleMovementComponent) AxisValue)
  (Variables|Default|SetLast_Gas (Math|Float|Absolute(Float) AxisValue)))

(event Input|AxisEvents|InputAxisSteering
  (params (AxisValue :type Float%20%28single-precision%29))
  ;[1 1 1] Steering
  (Class|ChaosVehicleMovementComponent|SetSteeringInput (Variables|Default|GetVehicleMovementComponent) AxisValue))

(event Input|MouseEvents|MouseX
  (params (AxisValue :type Float%20%28single-precision%29))
  (bind _mesh (Variables|Character|GetMesh))
  (bind _springarm (Variables|Default|GetSpringArm))
  (bind _springarm_2 (Variables|Default|GetSpringArm))
  (bind _returnvalue (Components|GetOwner _springarm))
  (bind _returnvalue_2 (Components|GetOwner _mesh))
  (bind _returnvalue_3 (Transformation|GetActorRotation _returnvalue))
  (bind _returnvalue_4 (Transformation|GetActorRotation _returnvalue_2))
  (bind _result (Math|Interpolation|Ease "Linear" 0.0 _returnvalue_3 _returnvalue_4 true))
  ;[1 1 1] Camera Control
  (if (and (<= (Math|Float|Absolute(Float) AxisValue) 0.1) (<= (Math|Float|Absolute(Float) (stale Input|MouseEvents|MouseY AxisValue)) 0.1))
    (if (>= (Variables|Default|GetCamera%20Movement%20Delta) 2.5)
      (Transformation|SetRelativeRotation (Variables|Default|GetSpringArm) (Math|Rotator|MakeRotator (.roll _result) (- (.pitch _result) 2e+01) (.yaw _result)) false false)
      (Variables|Default|SetCamera%20Movement%20Delta 2.5))
    (else
      (Transformation|AddRelativeRotation _springarm_2 (Math|Rotator|MakeRotator 0.0 0.0 AxisValue) false false)
      (Transformation|AddRelativeRotation _springarm_2 (Math|Rotator|MakeRotator 0.0 (stale Input|MouseEvents|MouseY AxisValue) 0.0) false false)
      (Variables|Default|SetCamera%20Movement%20Delta 0.0))))

(event Input|MouseEvents|MouseY
  (params (AxisValue :type Float%20%28single-precision%29))
  (bind _mesh (Variables|Character|GetMesh))
  (bind _springarm (Variables|Default|GetSpringArm))
  (bind _springarm_2 (Variables|Default|GetSpringArm))
  (bind _returnvalue (Components|GetOwner _springarm))
  (bind _returnvalue_2 (Components|GetOwner _mesh))
  (bind _returnvalue_3 (Transformation|GetActorRotation _returnvalue))
  (bind _returnvalue_4 (Transformation|GetActorRotation _returnvalue_2))
  (bind _result (Math|Interpolation|Ease "Linear" 0.0 _returnvalue_3 _returnvalue_4 true))
  ;[1 1 1] Camera Control
  (if (and (<= (Math|Float|Absolute(Float) (stale Input|MouseEvents|MouseX AxisValue)) 0.1) (<= (Math|Float|Absolute(Float) AxisValue) 0.1))
    (if (>= (Variables|Default|GetCamera%20Movement%20Delta) 2.5)
      (Transformation|SetRelativeRotation (Variables|Default|GetSpringArm) (Math|Rotator|MakeRotator (.roll _result) (- (.pitch _result) 2e+01) (.yaw _result)) false false)
      (Variables|Default|SetCamera%20Movement%20Delta 2.5))
    (else
      (Transformation|AddRelativeRotation _springarm_2 (Math|Rotator|MakeRotator 0.0 0.0 (stale Input|MouseEvents|MouseX AxisValue)) false false)
      (Transformation|AddRelativeRotation _springarm_2 (Math|Rotator|MakeRotator 0.0 AxisValue 0.0) false false)
      (Variables|Default|SetCamera%20Movement%20Delta 0.0))))

(fn ConstructionScript)