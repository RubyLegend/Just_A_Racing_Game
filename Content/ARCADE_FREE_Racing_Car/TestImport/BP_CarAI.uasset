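; Wheeled vehicle Blueprint for a drivable car; despite its AI name, it holds only input-driven control, with no AI logic.
; Input axes feed throttle, steering and brake to the vehicle movement component, while the handbrake also toggles rear lights and their material.
; Mouse input rotates the spring arm camera, which resets behind the car after an idle delay.
; A dynamic material created at construction displays forward speed on the speedometer each tick.
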(event EventTick
  (params (DeltaSeconds :type Float%20%28single-precision%29))
  ;[1 1 1] Modify speed on speedometer
  (Rendering|Material|SetScalarParameterValue (Variables|Default|GetSpeedometer_Value) "Speed" (/ (Math|Float|Absolute(Float) (Vehicle|GetForwardSpeed (Variables|Default|GetVehicleMovementComponent))) 27.778) :!class /Script/Engine.MaterialInstanceDynamic)
  (bind _output_get (Variables|Default|SetCamera%20Movement%20Delta (+ DeltaSeconds (stale _output_get)))))

(event Input|ActionEvents|InputActionHandBrake
  (params (Key :type Key%20Structure))
  (bind _vehiclemovementcomponent (Variables|Default|GetVehicleMovementComponent))
  (bind _mesh (Variables|Character|GetMesh))
  (bind _rl_light (Variables|Default|GetRL%20Light))
  ;[1 1 1] HandBrake
  (:Pressed
    (Class|ChaosVehicleMovementComponent|SetHandbrakeInput _vehiclemovementcomponent true)
    (Rendering|Material|SetMaterial _mesh 1 "/Game/ARCADE_FREE_Racing_Car/TestImport/BackLights_on.BackLights_on")
    (Rendering|SetVisibility _rl_light true false))
  (:Released
    (Class|ChaosVehicleMovementComponent|SetHandbrakeInput _vehiclemovementcomponent false)
    (Rendering|Material|SetMaterial _mesh 1 "/Game/ARCADE_FREE_Racing_Car/TestImport/BackLights_off.BackLights_off")
    (Rendering|SetVisibility _rl_light false false)))

(event Input|AxisEvents|InputAxisGas
  (params (AxisValue :type Float%20%28single-precision%29))
  ;[1 1 1] Gas
  (Class|ChaosVehicleMovementComponent|SetThrottleInput (Variables|Default|GetVehicleMovementComponent) AxisValue))

(event Input|AxisEvents|InputAxisReverseGas
  (params (AxisValue :type Float%20%28single-precision%29))
  ;[1 1 1] Gas
  (Class|ChaosVehicleMovementComponent|SetBrakeInput (Variables|Default|GetVehicleMovementComponent) AxisValue))

(event Input|AxisEvents|InputAxisSteering
  (params (AxisValue :type Float%20%28single-precision%29))
  ;[1 1 1] Steering
  (Class|ChaosVehicleMovementComponent|SetSteeringInput (Variables|Default|GetVehicleMovementComponent) AxisValue))

(event Input|MouseEvents|MouseX
  (params (AxisValue :type Float%20%28single-precision%29))
  (bind _mesh (Variables|Character|GetMesh))
  (bind _springarm (Variables|Default|GetSpringArm))
  (bind _springarm_2 (Variables|Default|GetSpringArm))
  (bind _returnvalue (Components|GetOwner _springarm))
  (bind _returnvalue_2 (Components|GetOwner _mesh))
  (bind _returnvalue_3 (Transformation|GetActorRotation _returnvalue))
  (bind _returnvalue_4 (Transformation|GetActorRotation _returnvalue_2))
  (bind _result (Math|Interpolation|Ease "Linear" 0.0 _returnvalue_3 _returnvalue_4 true))
  ;[1 1 1] Camera Control
  (if (and (<= (Math|Float|Absolute(Float) AxisValue) 0.1) (<= (Math|Float|Absolute(Float) (stale Input|MouseEvents|MouseY AxisValue)) 0.1))
    (if (>= (Variables|Default|GetCamera%20Movement%20Delta) 2.5)
      (Transformation|SetRelativeRotation (Variables|Default|GetSpringArm) (Math|Rotator|MakeRotator (.roll _result) (- (.pitch _result) 2e+01) (.yaw _result)) false false)
      (Variables|Default|SetCamera%20Movement%20Delta 2.5))
    (else
      (Transformation|AddRelativeRotation _springarm_2 (Math|Rotator|MakeRotator 0.0 0.0 AxisValue) false false)
      (Transformation|AddRelativeRotation _springarm_2 (Math|Rotator|MakeRotator 0.0 (stale Input|MouseEvents|MouseY AxisValue) 0.0) false false)
      (Variables|Default|SetCamera%20Movement%20Delta 0.0))))

(event Input|MouseEvents|MouseY
  (params (AxisValue :type Float%20%28single-precision%29))
  (bind _mesh (Variables|Character|GetMesh))
  (bind _springarm (Variables|Default|GetSpringArm))
  (bind _springarm_2 (Variables|Default|GetSpringArm))
  (bind _returnvalue (Components|GetOwner _springarm))
  (bind _returnvalue_2 (Components|GetOwner _mesh))
  (bind _returnvalue_3 (Transformation|GetActorRotation _returnvalue))
  (bind _returnvalue_4 (Transformation|GetActorRotation _returnvalue_2))
  (bind _result (Math|Interpolation|Ease "Linear" 0.0 _returnvalue_3 _returnvalue_4 true))
  ;[1 1 1] Camera Control
  (if (and (<= (Math|Float|Absolute(Float) (stale Input|MouseEvents|MouseX AxisValue)) 0.1) (<= (Math|Float|Absolute(Float) AxisValue) 0.1))
    (if (>= (Variables|Default|GetCamera%20Movement%20Delta) 2.5)
      (Transformation|SetRelativeRotation (Variables|Default|GetSpringArm) (Math|Rotator|MakeRotator (.roll _result) (- (.pitch _result) 2e+01) (.yaw _result)) false false)
      (Variables|Default|SetCamera%20Movement%20Delta 2.5))
    (else
      (Transformation|AddRelativeRotation _springarm_2 (Math|Rotator|MakeRotator 0.0 0.0 (stale Input|MouseEvents|MouseX AxisValue)) false false)
      (Transformation|AddRelativeRotation _springarm_2 (Math|Rotator|MakeRotator 0.0 AxisValue 0.0) false false)
      (Variables|Default|SetCamera%20Movement%20Delta 0.0))))

(fn ConstructionScript
  (bind _returnvalue (Rendering|Material|CreateDynamicMaterialInstance (Variables|Default|GetPlane) 0 "/Game/UI/MI_Speedometer.MI_Speedometer" "None" :!class /Script/Engine.PrimitiveComponent))
  (Variables|Default|SetSpeedometer_Value _returnvalue))